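; BP_EnemyHit is an animation notify that applies a melee hit to the player, filed under the Grandmother enemy character.
; When it fires, it casts player character 0 to BaseCharacter and measures that character's distance to the owner of the animated mesh.
; Within a fixed radius it calls TakeDamage with a hardcoded amount, using only distance with no trace or facing check.
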(fn `Received_Notify`
  (params (MeshComp :type "SkeletalMeshComponent Object Reference") (Animation :type "AnimSequenceBase Object Reference"))
  (returns (ReturnValue :type Boolean))
  (bind _returnvalue (`GameplayStatics.GetPlayerCharacter` 0))
  (bind _asbase_character (cast `BaseCharacter` _returnvalue))
  (if (< (`KismetMathLibrary.VSize` (- (`Actor.K2_GetActorLocation` _returnvalue) (`Actor.K2_GetActorLocation` (`ActorComponent.GetOwner` MeshComp)))) 300.0)
    (`BaseCharacter.TakeDamage` _asbase_character 25.0)
    (return false)))