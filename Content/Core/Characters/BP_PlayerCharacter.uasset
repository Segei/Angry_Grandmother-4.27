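; BP_PlayerCharacter is the first-person player character, handling movement, look, jump, and weapon fire and reload input.
; BeginPlay creates health, score and life widgets and binds to OnSetWeapon.
; The first weapon set adds ammo and crosshair widgets through a handler that unbinds itself.
; Every weapon set moves the OnShootRifle binding to the new weapon, so each shot plays the rifle fire montage.
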(event `CustomEvent` :!signature `self.OnSetWeapon`
  (params (Player :type "PlayerCharacter Object Reference"))
  (remove `self.OnSetWeapon` Player (delegate `CustomEvent`))
  (bind _returnvalue (`|CreateWidget` "/Game/Core/Widgets/UIBP_Ammo.UIBP_Ammo_C"))
  (`UserWidget.AddToViewport` _returnvalue 0)
  (bind _returnvalue_2 (`|CreateWidget` "/Game/Core/Widgets/UIBP_CrossHair.UIBP_CrossHair_C"))
  (`UserWidget.AddToViewport` _returnvalue_2 0))

(event `self.ReceiveBeginPlay`
  (add `self.OnSetWeapon` (delegate `OnSetWeapon_Event_0`))
  (add `self.OnSetWeapon` (delegate `CustomEvent`))
  (bind _returnvalue (`|CreateWidget` "/Game/Core/Widgets/UIBP_Health.UIBP_Health_C"))
  (`UserWidget.AddToViewport` _returnvalue 0)
  (bind _returnvalue_2 (`|CreateWidget` "/Game/Core/Widgets/UIBP_Score.UIBP_Score_C"))
  (`UserWidget.AddToViewport` _returnvalue_2 0)
  (bind _returnvalue_3 (`|CreateWidget` "/Game/Core/Widgets/UIBP_Life.UIBP_Life_C"))
  (`UserWidget.AddToViewport` _returnvalue_3 0))

(event `InputAxis|LookUp`
  (params (AxisValue :type "Float (single-precision)"))
  (`self.AddControllerPitchInput` AxisValue))

(event `OnSetWeapon_Event_0` :!signature `self.OnSetWeapon`
  (params (Player :type "PlayerCharacter Object Reference"))
  (bind _cachedweapon (`self.CachedWeapon`))
  (`/Engine/EditorBlueprintResources/StandardMacros.IsValid` _cachedweapon
    (:`Is Valid`
      (remove `RangeWeapon.OnShootRifle` _cachedweapon (delegate `OnShootRifle_Event_0`)))
    (:`Is Not Valid`
      _))
  (bind _output_get (set `self.CachedWeapon` (`PlayerCharacter.CurrentWeapon` Player)))
  (add `RangeWeapon.OnShootRifle` _output_get (delegate `OnShootRifle_Event_0`)))

(event `InputAxis|Turn`
  (params (AxisValue :type "Float (single-precision)"))
  (`self.AddControllerYawInput` AxisValue))

(event `OnShootRifle_Event_0`
  (`|PlayMontage` (`self.MeshComponent`) "/Game/Core/Characters/FirstPerson/Animations/FP_Rifle_Fire_Montage.FP_Rifle_Fire_Montage"))

(event `InputAxis|MoveForward`
  (params (AxisValue :type "Float (single-precision)"))
  (`self.AddMovementInput` (`self.GetActorForwardVector`) AxisValue))

(event `InputAxis|MoveRight`
  (params (AxisValue :type "Float (single-precision)"))
  (`self.AddMovementInput` (`self.GetActorRightVector`) AxisValue))

(event `InputAction|Reload`
  (params (Key :type "Key Structure"))
  (bind _currentweapon (`self.CurrentWeapon`))
  (:`Pressed`
    (`/Engine/EditorBlueprintResources/StandardMacros.IsValid` _currentweapon
      (:`Is Valid`
        (`RangeWeapon.StartReload` _currentweapon)))))

(event `InputAxis|Fire`
  (params (AxisValue :type "Float (single-precision)"))
  (bind _currentweapon (`self.CurrentWeapon`))
  (`/Engine/EditorBlueprintResources/StandardMacros.IsValid` _currentweapon
    (:`Is Valid`
      (if (> AxisValue 0.0)
        (`RangeWeapon.StartShooting` _currentweapon)
        (else
          (`RangeWeapon.EndShooting` _currentweapon))))))

(event `InputAction|Jump`
  (params (Key :type "Key Structure"))
  (:`Pressed`
    (`self.Jump`)))

(fn `UserConstructionScript`)