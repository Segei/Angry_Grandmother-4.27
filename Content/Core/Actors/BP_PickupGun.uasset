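; BP_PickupGun is a rotating world pickup that gives the player a ranged weapon on overlap.
; On BeginPlay it spawns its configured weapon class and attaches that weapon to its sphere.
; Overlap attaches the cached weapon to the player's GripPoint socket and sets it as current.
; Any weapon the player already held becomes the new pickup in a swap; otherwise the pickup destroys itself.
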(event `self.ReceiveBeginPlay`
  (bind _returnvalue (`|SpawnActorFromClass` (`self.WeaponSpawnClass`) (`self.GetTransform`) "AlwaysSpawn" "OverrideRootScale" null null))
  (bind _asrange_weapon (cast `RangeWeapon` _returnvalue))
  (`self.Set Weapon To Pickup` _asrange_weapon))

(event `self.Sphere.OnComponentBeginOverlap`
  (params (OverlappedComponent :type "PrimitiveComponent Object Reference") (OtherActor :type "Actor Object Reference") (OtherComp :type "PrimitiveComponent Object Reference") (OtherBodyIndex :type Integer) (bFromSweep :type Boolean) (SweepResult :type "HitResult Structure (by ref)"))
  (bind _firstpersoncharacterreference (`self.FirstPersonCharacterReference`))
  (bind _tempweapon (`self.TempWeapon`))
  (bind _currentweapon (`PlayerCharacter.CurrentWeapon` _firstpersoncharacterreference))
  (bind _asplayer_character (cast `PlayerCharacter` OtherActor))
  (set `self.FirstPersonCharacterReference` _asplayer_character)
  (`/Engine/EditorBlueprintResources/StandardMacros.IsValid` _currentweapon
    (:`Is Valid`
      (set `self.TempWeapon` _currentweapon))
    (:`Is Not Valid`
      _))
  (`self.SetOwner` (`self.CachedWeapon`) _firstpersoncharacterreference)
  (`self.K2_AttachToComponent` (`self.CachedWeapon`) (`PlayerCharacter.MeshComponent` _firstpersoncharacterreference) "GripPoint" "SnapToTarget" "SnapToTarget" "SnapToTarget" true)
  (`PlayerCharacter.SetWeapon` (`self.FirstPersonCharacterReference`) (`self.CachedWeapon`))
  (`/Engine/EditorBlueprintResources/StandardMacros.IsValid` _tempweapon
    (:`Is Valid`
      (`self.Set Weapon to Pickup` _tempweapon)
      (set `self.TempWeapon` null))
    (:`Is Not Valid`
      (`self.K2_DestroyActor`))))

(event `self.ReceiveTick`
  (params (DeltaSeconds :type "Float (single-precision)"))
  (`self.K2_AddActorWorldRotation` (struct :`Yaw` 1.0)))

(fn `Set Weapon To Pickup`
  (params (Weapon :type "RangeWeapon Object Reference"))
  (bind _output_get (set `self.CachedWeapon` Weapon))
  (`self.K2_AttachToComponent` _output_get (`self.Sphere`) "None" "SnapToTarget" "SnapToTarget" "SnapToTarget" true)
  (`self.SetOwner` _output_get self))

(fn `UserConstructionScript`)